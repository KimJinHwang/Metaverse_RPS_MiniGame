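; Player actor that steps around a 5x5 grid with the arrow keys and attacks monsters with Space.
; Move updates the clamped grid position in the PlayerInfo struct, converts it to world space at 110-unit spacing, faces that point and jumps there without sweeping.
; Attack calls OnDamaged on the first BP_Monster overlapping the capsule, or prints a failure message if the cast fails.
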(event `self.ReceiveBeginPlay`
  (`self.EnableInput` (`GameplayStatics.GetPlayerController` 0))
  (`self.K2_SetActorLocation` (0.0 0.0 50.0)))

(event `Key|Left`
  (params (Key :type "Key Structure"))
  (:`Pressed`
    (`self.Move` 0 -1)))

(event `Key|Right`
  (params (Key :type "Key Structure"))
  (:`Pressed`
    (`self.Move` 0 1)))

(event `Key|Up`
  (params (Key :type "Key Structure"))
  (:`Pressed`
    (`self.Move` 1)))

(event `Key|Down`
  (params (Key :type "Key Structure"))
  (:`Pressed`
    (`self.Move` -1)))

(event `Key|SpaceBar`
  (params (Key :type "Key Structure"))
  (:`Pressed`
    (`self.Attack`)))

(fn `Attack`
  (bind _asbp_monster (cast `/Game/BP_Monster` (`|GetArrayItem` (`PrimitiveComponent.GetOverlappingActors` (`self.CapsuleComponent`) "/Game/BP_Monster.BP_Monster_C")))
    (:`then`
      (`/Game/BP_Monster.On Damaged` _asbp_monster))
    (:`CastFailed`
      (`KismetSystemLibrary.PrintText` "실패"))))

(fn `Move`
  (params (X :type Integer) (Y :type Integer))
  (bind (_playerinfo_name _playerinfo_positionx _playerinfo_positiony _playerinfo_gold) (break `/Game/Structures/PlayerInfo` (`self.PlayerInfo`)))
  (bind _output_get (set `self.PlayerInfo` (make `/Game/Structures/PlayerInfo` _playerinfo_name (`KismetMathLibrary.Clamp` (+ _playerinfo_positionx X) 0 4) (`KismetMathLibrary.Clamp` (+ _playerinfo_positiony Y) 0 4) _playerinfo_gold)))
  (bind _returnvalue (`KismetMathLibrary.MakeVector` (`KismetMathLibrary.Conv_IntToDouble` (* (`.PositionX_5_486824AA4BD153AC7B3C4AB33612F8ED` (break `/Game/Structures/PlayerInfo` _output_get)) 110)) (`KismetMathLibrary.Conv_IntToDouble` (* (`.PositionY_7_0B3FCE334DDD279827F7A58F2D5887BC` (break `/Game/Structures/PlayerInfo` _output_get)) 110)) 50.0))
  (`self.K2_SetActorRotation` (`KismetMathLibrary.MakeRotFromX` (`KismetMathLibrary.Vector_Normal2D` (- _returnvalue (`self.K2_GetActorLocation`)))))
  (`self.K2_SetActorLocation` _returnvalue))

(fn `UserConstructionScript`)