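; Game mode that generates a randomized 5x5 tile board with monsters when play begins.
; It spawns BP_Tile actors into the Tilemap array, derives grid coordinates from each index, and positions tiles at fixed spacing.
; Each TileInfo gets a 20% monster chance and a random integer.
; A second sequence pass spawns a scaled-down BP_Monster above every tile flagged as having one.
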(event `self.ReceiveBeginPlay`
  (bind _tilemap (`self.Tilemap`))
  (`|ExecutionSequence`
    (:`then_0`
      ;[1 1 1] 타일맵 크기 설정
      (`KismetArrayLibrary.Array_Resize` _tilemap 25)
      ;[1 1 1] 타일 생성 (기본위치)
      (for (_ _array_index) _tilemap
        (bind _returnvalue (`|SpawnActorFromClass` "/Game/BP_Tile.BP_Tile_C" (`KismetMathLibrary.MakeTransform` (0.0 0.0 0.0)) "Undefined" "OverrideRootScale" null null))
        ;[1 1 1] 타일 데이터 셋팅
        (`KismetArrayLibrary.Array_Set` (`self.Tilemap`) _array_index _returnvalue)
        (bind _output_get (set `/Game/BP_Tile.TileInfo` (make `/Game/Structures/TileInfo` (/ _array_index 5) (mod _array_index 5) (< (`KismetMathLibrary.RandomInteger` 100) 20) (`KismetMathLibrary.RandomInteger` 101)) (`|GetArrayItem` (`self.Tilemap`) _array_index)))
        (bind _returnvalue_location (`KismetMathLibrary.BreakTransform` (`KismetMathLibrary.MakeTransform` (`KismetMathLibrary.MakeVector` (`KismetMathLibrary.Conv_IntToDouble` (* (break `/Game/Structures/TileInfo` _output_get) 110)) (`KismetMathLibrary.Conv_IntToDouble` (* (`.IdY_4_5CCCA53B41C4253CDF8334A6CD769BF5` (break `/Game/Structures/TileInfo` _output_get)) 110)) 20.0))))
        ;[1 1 1] 타일 실제 위치 설정
        (`self.K2_SetActorLocation` (`|GetArrayItem` (`self.Tilemap`) _array_index) _returnvalue_location false false)))
    (:`then_1`
      (for _array_element (`self.Tilemap`)
        (bind (_tileinfo_idx _tileinfo_idy _tileinfo_bexistmonster) (break `/Game/Structures/TileInfo` (`/Game/BP_Tile.TileInfo` _array_element)))
        (if _tileinfo_bexistmonster
          (`|SpawnActorFromClass` "/Game/BP_Monster.BP_Monster_C" (`KismetMathLibrary.MakeTransform` (`KismetMathLibrary.MakeVector` (`KismetMathLibrary.Conv_IntToDouble` (* _tileinfo_idx 110)) (`KismetMathLibrary.Conv_IntToDouble` (* _tileinfo_idy 110)) 50.0) (struct :`Yaw` 180.0) (0.6 0.6 0.6)) "Undefined" "OverrideRootScale" null null))))))

(fn `UserConstructionScript`)